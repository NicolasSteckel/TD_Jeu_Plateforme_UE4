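; BP_WindBoxes is a wind volume that pushes the first-person player character along an arrow's direction.
; BeginPlay caches player 0's character, and the Tick event launches it along the arrow's forward vector scaled by ForcePoussée, overriding its velocity.
; Any WindZone overlap starts a short non-looping timer bound to Tick, and ending the overlap clears that timer.
; Tick itself has no overlap check.
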(event `self.WindZone.OnComponentBeginOverlap`
  (params (OverlappedComponent :type "PrimitiveComponent Object Reference") (OtherActor :type "Actor Object Reference") (OtherComp :type "PrimitiveComponent Object Reference") (OtherBodyIndex :type Integer) (bFromSweep :type Boolean) (SweepResult :type "HitResult Structure (by ref)"))
  (bind _returnvalue (`KismetSystemLibrary.K2_SetTimerDelegate` (delegate `Tick`) 0.03333)))

(event `Tick`
  (`Character.LaunchCharacter` (`self.Char`) (* (`SceneComponent.GetForwardVector` (`self.Arrow`)) (`self.Force Poussée`)) true true))

(event `self.WindZone.OnComponentEndOverlap`
  (params (OverlappedComponent :type "PrimitiveComponent Object Reference") (OtherActor :type "Actor Object Reference") (OtherComp :type "PrimitiveComponent Object Reference") (OtherBodyIndex :type Integer))
  (`KismetSystemLibrary.K2_ClearAndInvalidateTimerHandle` (stale `self.WindZone.OnComponentBeginOverlap` _returnvalue)))

(event `self.ReceiveBeginPlay`
  (bind _asfirst_person_character (cast `/Game/FirstPersonBP/Blueprints/FirstPersonCharacter` (`GameplayStatics.GetPlayerCharacter` 0)))
  (set `self.Char` _asfirst_person_character))

(fn `UserConstructionScript`)