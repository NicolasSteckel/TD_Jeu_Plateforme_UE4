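; Level-end trigger that shows the end screen when an actor overlaps it and no collectables remain in the level.
; On overlap it counts all BP_Collectables actors, with no check on which actor entered.
; If none are left, it adds EcranFin_widget to the viewport, shows the mouse cursor and switches the first player controller to UI-only input.
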(event `self.ReceiveActorBeginOverlap`
  (params (OtherActor :type "Actor Object Reference"))
  (bind _returnvalue (`GameplayStatics.GetPlayerController` 0))
  (if (not (`self.Is any item remaining`))
    (bind _returnvalue_2 (`|CreateWidget` "/Game/Blueprints/Widget/EcranFin_widget.EcranFin_widget_C" _returnvalue))
    (`UserWidget.AddToViewport` _returnvalue_2 0)
    (set `PlayerController.bShowMouseCursor` true _returnvalue)
    (`WidgetBlueprintLibrary.SetInputMode_UIOnlyEx` _returnvalue _returnvalue_2)))

(fn `Is any item remaining`
  (returns (ReturnValue :type Boolean))
  (bind _outactors (`GameplayStatics.GetAllActorsOfClass` "/Game/Blueprints/Collectables/BP_Collectables.BP_Collectables_C"))
  (return (> (`KismetMathLibrary.Conv_IntToByte` (`KismetArrayLibrary.Array_Length` _outactors)) 0)))

(fn `UserConstructionScript`)